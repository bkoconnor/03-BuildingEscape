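; Cabinet Blueprint that swings open and closed in response to OpenDoor open and close events.
; It stores its initial rotation on BeginPlay, then a timeline adds an animated yaw angle to it and rotates the whole actor.
; A timeline event track plays a door lock sound at the actor's location, and closing reverses the same timeline.
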(event OnClose(OpenDoor)
  (bind _open_angle (Timeline|Timeline_0 Reverse)
    (:Update
      (Transformation|SetActorRotation (Math|Rotator|CombineRotators (Math|Rotator|MakeRotator 0.0 0.0 _open_angle) (Variables|Default|GetInitial%20Rotation))))
    (:Sound%20Timing
      (Audio|PlaySoundatLocation "/Game/Audio/door-lock.door-lock" (Transformation|GetActorLocation)))))

(event OnOpen(OpenDoor)
  (bind _open_angle (Timeline|Timeline_0 Play)
    (:Update
      (Transformation|SetActorRotation (Math|Rotator|CombineRotators (Math|Rotator|MakeRotator 0.0 0.0 _open_angle) (Variables|Default|GetInitial%20Rotation))))
    (:Sound%20Timing
      (Audio|PlaySoundatLocation "/Game/Audio/door-lock.door-lock" (Transformation|GetActorLocation)))))

(event EventBeginPlay
  (Variables|Default|SetInitial%20Rotation (Transformation|GetActorRotation)))

(fn ConstructionScript)